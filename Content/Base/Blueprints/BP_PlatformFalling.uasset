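; BP_PlatformFalling is a platform actor that rises to a target height and falls away, starting its fall state eight seconds after BeginPlay.
; While Rising, which takes priority, Tick eases Z toward TargetPosition with FInterpTo and clears the flag once nearly there.
; While Falling, it accumulates downward FallVelocity and adds it per frame without delta scaling or sweep.
; Rising and TargetPosition are not set within this Blueprint.
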(event `self.ReceiveBeginPlay`
  (`KismetSystemLibrary.Delay` 8.0)
  (set `self.Falling` true))

(event `self.ReceiveTick`
  (params (DeltaSeconds :type "Float (single-precision)"))
  (bind (_returnvalue_x _returnvalue_y) (`KismetMathLibrary.BreakVector` (`self.K2_GetActorLocation`)))
  (bind (_returnvalue_x_2 _returnvalue_y_2 _returnvalue_z) (`KismetMathLibrary.BreakVector` (`self.K2_GetActorLocation`)))
  (bind (_targetposition_x _targetposition_y _targetposition_z) (`KismetMathLibrary.BreakVector` (`self.TargetPosition`)))
  (bind _returnvalue (`KismetMathLibrary.MakeVector` _returnvalue_x _returnvalue_y (`KismetMathLibrary.FInterpTo` _returnvalue_z _targetposition_z DeltaSeconds 10.0)))
  (if (`self.Rising`)
    (`self.K2_SetActorLocation` _returnvalue)
    (`/Engine/EditorBlueprintResources/StandardMacros.CompareFloat` (`KismetMathLibrary.Vector_Distance` _returnvalue (`self.TargetPosition`)) 1.0
      (:`<`
        (set `self.Rising` false)))
    (elif (`self.Falling`)
      (bind _output_get (set `self.FallVelocity` (+ (`self.FallVelocity`) (`KismetMathLibrary.MakeVector` 0.0 0.0 (* (`GameplayStatics.GetWorldDeltaSeconds`) -10.0)))))
      (`self.K2_SetActorLocation` (+ _output_get (`self.K2_GetActorLocation`))))))

(fn `UserConstructionScript`)