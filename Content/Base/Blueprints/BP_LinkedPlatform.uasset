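; BP_LinkedPlatform is a platform in a linked path that, when hit by the player character, activates its next platforms and deactivates previous ones.
; Construction syncs links both ways and draws arrows to next platforms, while SpawnNextPlatform adds a linked copy.
; Active platforms toggle visibility and collision.
; At BeginPlay, an initially active platform walks the graph breadth-first and joins platforms with spline meshes, using averaged link directions as tangents.
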(event `self.ReceiveBeginPlay`
  (`self.SetPlatformActivity` (`self.CurrentlyActive`))
  (`self.CleanPlatformArrays`)
  (if (`self.CurrentlyActive`)
    (`self.GenerateSplineTrail`)))

(event `self.StaticMesh.OnComponentHit`
  (params (HitComponent :type "PrimitiveComponent Object Reference") (OtherActor :type "Actor Object Reference") (OtherComp :type "PrimitiveComponent Object Reference") (NormalImpulse :type "Vector Structure") (Hit :type "HitResult Structure (by ref)"))
  (cast `/Game/Base/Blueprints/FirstPersonCharacter` OtherActor)
  (for _array_element (`self.NextPlatforms`)
    (`self.SetPlatformActivity` _array_element true))
  (for _array_element_2 (`self.PreviousPlatforms`)
    (`self.SetPlatformActivity` _array_element_2 false)))

(fn `CleanPlatformArrays`
  (bind (_arrayindex _arrayelement) (`/Engine/EditorBlueprintResources/StandardMacros.ReverseForEachLoop` (`self.NextPlatforms`))
    (:`LoopBody`
      (`/Engine/EditorBlueprintResources/StandardMacros.IsValid` _arrayelement
        (:`Is Not Valid`
          (`KismetArrayLibrary.Array_Remove` (`self.NextPlatforms`) _arrayindex))))
    (:`Completed`
      (bind (_arrayindex_2 _arrayelement_2) (`/Engine/EditorBlueprintResources/StandardMacros.ReverseForEachLoop` (`self.PreviousPlatforms`))
        (:`LoopBody`
          (`/Engine/EditorBlueprintResources/StandardMacros.IsValid` _arrayelement_2
            (:`Is Not Valid`
              (`KismetArrayLibrary.Array_Remove` (`self.PreviousPlatforms`) _arrayindex_2))))
        (:`Completed`
          (`self.UpdateArrows` false))))))

(fn `GenerateSplineTrail`
  (locals (PlatformsToCheck :type "Array of /Game/Base/Blueprints/BP_LinkedPlatform Object Reference") (PlatformList :type "Array of /Game/Base/Blueprints/BP_LinkedPlatform Object Reference") (NewPlatforms :type "Array of /Game/Base/Blueprints/BP_LinkedPlatform Object Reference") (SplineData :type "Array of /Game/Base/Blueprints/ST_LinkedPlatformSplineData Structure") (NewSplineData :type "/Game/Base/Blueprints/ST_LinkedPlatformSplineData Structure") (IncomingVectors :type "Array of Vector Structure") (OutgoingVectors :type "Array of Vector Structure"))
  (set `local.PlatformList` (`|MakeArray` self :!type "/Game/Base/Blueprints/BP_LinkedPlatform Object Reference"))
  (`KismetArrayLibrary.Array_Append` (`local.PlatformList`) (`self.NextPlatforms`))
  (set `local.PlatformsToCheck` (`self.NextPlatforms`))
  (while (> (`KismetArrayLibrary.Array_Length` (`local.PlatformsToCheck`)) 0)
    (for _array_element (`local.PlatformsToCheck`)
      (for _array_element_2 (`/Game/Base/Blueprints/BP_LinkedPlatform.NextPlatforms` _array_element)
        (`KismetArrayLibrary.Array_AddUnique` (`local.NewPlatforms`) _array_element_2)))
    (`KismetArrayLibrary.Array_Clear` (`local.PlatformsToCheck`))
    (for _array_element_3 (`local.NewPlatforms`)
      (if (== (`KismetArrayLibrary.Array_Find` (`local.PlatformList`) _array_element_3) -1)
        (`KismetArrayLibrary.Array_AddUnique` (`local.PlatformsToCheck`) _array_element_3)
        (`KismetArrayLibrary.Array_AddUnique` (`local.PlatformList`) _array_element_3)))
    (`KismetArrayLibrary.Array_Clear` (`local.NewPlatforms`)))
  (for _array_element_4 (`local.PlatformList`)
    (`KismetSystemLibrary.PrintString` (`KismetSystemLibrary.GetDisplayName` _array_element_4))
    (for _array_element_5 (`/Game/Base/Blueprints/BP_LinkedPlatform.PreviousPlatforms` _array_element_4)
      (bind _returnvalue (`self.K2_GetActorLocation` _array_element_4))
      (`KismetArrayLibrary.Array_Add` (`local.IncomingVectors`) (`KismetMathLibrary.GetDirectionUnitVector` (`self.K2_GetActorLocation` _array_element_5) _returnvalue)))
    (for _array_element_6 (`/Game/Base/Blueprints/BP_LinkedPlatform.NextPlatforms` _array_element_4)
      (`KismetArrayLibrary.Array_Add` (`local.OutgoingVectors`) (`KismetMathLibrary.GetDirectionUnitVector` _returnvalue (`self.K2_GetActorLocation` _array_element_6))))
    (`KismetArrayLibrary.Array_Append` (`local.IncomingVectors`) (`local.OutgoingVectors`))
    (set `/Game/Base/Blueprints/BP_LinkedPlatform.Direction` (`KismetMathLibrary.GetVectorArrayAverage` (`local.IncomingVectors`)) _array_element_4))
  (for _array_element_7 (`local.PlatformList`)
    (for _array_element_8 (`/Game/Base/Blueprints/BP_LinkedPlatform.NextPlatforms` _array_element_7)
      (bind _returnvalue_2 (`AddComponent|NODE_AddSplineMeshComponent-0` :`self` _array_element_7))
      (bind _returnvalue_3 (`self.K2_GetActorLocation` _array_element_7))
      (`SplineMeshComponent.SetStartPosition` _returnvalue_2 _returnvalue_3 true)
      (bind _returnvalue_4 (`self.K2_GetActorLocation` _array_element_8))
      (`SplineMeshComponent.SetEndPosition` _returnvalue_2 _returnvalue_4 true)
      (bind _returnvalue_5 (`KismetMathLibrary.Vector_Distance` _returnvalue_4 _returnvalue_3))
      (`SplineMeshComponent.SetStartTangent` _returnvalue_2 (* (`/Game/Base/Blueprints/BP_LinkedPlatform.Direction` _array_element_7) _returnvalue_5) true)
      (`SplineMeshComponent.SetEndTangent` _returnvalue_2 (* (`/Game/Base/Blueprints/BP_LinkedPlatform.Direction` _array_element_8) _returnvalue_5) true))))

(fn `SetPlatformActivity`
  (params (IsActive :type Boolean))
  (set `self.CurrentlyActive` IsActive)
  (`SceneComponent.SetVisibility` (`self.DefaultSceneRoot`) (`self.CurrentlyActive`) true)
  (`self.SetActorEnableCollision` (`self.CurrentlyActive`)))

(fn `SpawnNextPlatform`
  (locals (NewPlatform :type "/Game/Base/Blueprints/BP_LinkedPlatform Object Reference"))
  (bind _returnvalue_location (`KismetMathLibrary.BreakTransform` (`self.GetTransform`)))
  (bind _returnvalue (`|SpawnActorFromClass` "BP_LinkedPlatform_C" (`KismetMathLibrary.MakeTransform` (+ _returnvalue_location (200.0 0.0 0.0))) "Undefined" "OverrideRootScale" null null))
  (set `local.NewPlatform` _returnvalue)
  (set `/Game/Base/Blueprints/BP_LinkedPlatform.PreviousPlatforms` (`|MakeArray` self :!type "/Game/Base/Blueprints/BP_LinkedPlatform Object Reference") (`local.NewPlatform`))
  (`KismetArrayLibrary.Array_Add` (`self.NextPlatforms`) (`local.NewPlatform`))
  (set `/Game/Base/Blueprints/BP_LinkedPlatform.StaticMeshAsset` (`self.StaticMeshAsset`) (`local.NewPlatform`))
  (set `/Game/Base/Blueprints/BP_LinkedPlatform.MaterialAsset` (`self.MaterialAsset`) (`local.NewPlatform`)))

(fn `UpdateArrows`
  (params (FirstCall :type Boolean))
  (locals (CurrentNextPlatform :type "/Game/Base/Blueprints/BP_LinkedPlatform Object Reference"))
  (bind _returnvalue (`self.K2_GetActorLocation`))
  (bind _returnvalue_2 (`self.K2_GetActorLocation` (`local.CurrentNextPlatform`)))
  (for _array_element (`self.K2_GetComponentsByClass` "/Script/Engine.ArrowComponent")
    (`ActorComponent.K2_DestroyComponent` _array_element))
  (for _array_element_2 (`self.NextPlatforms`)
    (bind _output_get (set `local.CurrentNextPlatform` _array_element_2))
    (`/Engine/EditorBlueprintResources/StandardMacros.IsValid` _output_get
      (:`Is Valid`
        (`AddComponent|NODE_AddArrowComponent-1` :`RelativeTransform` (`KismetMathLibrary.MakeTransform` (0.0 0.0 0.0) (`KismetMathLibrary.FindLookAtRotation` _returnvalue _returnvalue_2) (`KismetMathLibrary.MakeVector` (/ (`KismetMathLibrary.Vector_Distance` _returnvalue _returnvalue_2) 80.0) 5.0 5.0))))))
  (if (`local.FirstCall`)
    (for _array_element_3 (`self.PreviousPlatforms`)
      (`self.UpdateArrows` _array_element_3 false))))

(fn `UpdateOtherPlatforms`
  (for _array_element (`self.NextPlatforms`)
    (`KismetArrayLibrary.Array_AddUnique` (`/Game/Base/Blueprints/BP_LinkedPlatform.PreviousPlatforms` _array_element) self))
  (for _array_element_2 (`self.PreviousPlatforms`)
    (`KismetArrayLibrary.Array_AddUnique` (`/Game/Base/Blueprints/BP_LinkedPlatform.NextPlatforms` _array_element_2) self)))

(fn `UserConstructionScript`
  (`StaticMeshComponent.SetStaticMesh` (`self.StaticMesh`) (`self.StaticMeshAsset`))
  (`PrimitiveComponent.SetMaterial` (`self.StaticMesh`) 0 (`self.MaterialAsset`))
  (`self.UpdateOtherPlatforms`)
  (`self.UpdateArrows` true))