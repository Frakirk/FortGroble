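; A pillow actor that grows into a wide, flattened shape when play begins and pushes the first-person character on contact.
; A timeline drives the growth from a tiny starting scale.
; Its box overlap raises and lowers the character's NoDeathFields counter, apparently marking a safe zone, while mesh hits add amplified normal impulse to the character's velocity.
; Rotation-interpolation logic with debug prints is left unconnected and never runs.
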(event `self.ReceiveBeginPlay`
  (`self.SetActorScale3D` (0.1 0.1 0.1))
  (bind (_direction _scale) (`Timeline|GrowPillow` :!via `PlayFromStart`)
    (:`Update`
      (`self.SetActorScale3D` (* (2.0 2.0 0.5) _scale))
      (if (== (`KismetMathLibrary.VInterpTo` (`self.GetActorScale3D`) (1.0 1.0 1.0) (`GameplayStatics.GetWorldDeltaSeconds`) 1.0) (1.0 1.0 1.0))
        (`KismetSystemLibrary.K2_ClearTimer` null "GrowPillow")))
    (:`Finished`
      (`self.SetActorScale3D` (2.0 2.0 0.5)))))

(event `self.ReceiveTick`
  (params (DeltaSeconds :type "Float (single-precision)")))

(event `self.Box.OnComponentBeginOverlap`
  (params (OverlappedComponent :type "PrimitiveComponent Object Reference") (OtherActor :type "Actor Object Reference") (OtherComp :type "PrimitiveComponent Object Reference") (OtherBodyIndex :type Integer) (bFromSweep :type Boolean) (SweepResult :type "HitResult Structure (by ref)"))
  (bind _asfirst_person_character (cast `/Game/Base/Blueprints/FirstPersonCharacter` OtherActor))
  (`/Engine/EditorBlueprintResources/StandardMacros.IncrementInt` (`/Game/Base/Blueprints/FirstPersonCharacter.NoDeathFields` _asfirst_person_character)))

(event `self.Box.OnComponentEndOverlap`
  (params (OverlappedComponent :type "PrimitiveComponent Object Reference") (OtherActor :type "Actor Object Reference") (OtherComp :type "PrimitiveComponent Object Reference") (OtherBodyIndex :type Integer))
  (bind _asfirst_person_character (cast `/Game/Base/Blueprints/FirstPersonCharacter` OtherActor))
  (`/Engine/EditorBlueprintResources/StandardMacros.DecrementInt` (`/Game/Base/Blueprints/FirstPersonCharacter.NoDeathFields` _asfirst_person_character)))

(event `self.Mesh.OnComponentHit`
  (params (HitComponent :type "PrimitiveComponent Object Reference") (OtherActor :type "Actor Object Reference") (OtherComp :type "PrimitiveComponent Object Reference") (NormalImpulse :type "Vector Structure") (Hit :type "HitResult Structure (by ref)"))
  (bind _asfirst_person_character (cast `/Game/Base/Blueprints/FirstPersonCharacter` OtherActor))
  (bind _charactermovement (`Character.CharacterMovement` _asfirst_person_character))
  (set `MovementComponent.Velocity` (+ (* NormalImpulse 1000.0) (`MovementComponent.Velocity` _charactermovement)) _charactermovement))

(fn `UserConstructionScript`)